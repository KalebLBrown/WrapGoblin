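; Goblin enemy AI that wanders between random BP_EnemyInterestPoint actors and chases the player when PawnSensing spots them.
; A retriggerable delay slightly longer than the sensing interval clears the seeing flag once sightings stop.
; Tick then sends the goblin to the last recorded player location, and on arrival it resumes wandering after a short timer.
; Catching the player only prints a TODO.
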(event OnSeePawn(PawnSensing)
  (params (Pawn :type Pawn%20Object%20Reference))
  (Variables|Default|SetisSeeingPlayer true)
  (Development|PrintString "Seeing player!")
  (Utilities|FlowControl|Sequence
    (:then_0
      (CallFunction|FollowPLayer))
    (:then_1
      (Utilities|FlowControl|RetriggerableDelay (+ (Variables|/Script/AIModule.PawnSensingComponent|GetSensingInterval (Variables|Default|GetPawnSensing)) 0.1)) ; Delay until player isn't seen anymore
      (Variables|Default|SetisSeeingPlayer false)
      (Development|PrintString "No longer seeing player!"))))

(event Custom|FollowPlayer
  (bind _returnvalue (Game|GetPlayerCharacter 0))
  (if (Variables|Default|GetisSeeingPlayer)
    (AI|AIMoveTo self "0, 0, 0" _returnvalue 5.0 false
      (:then
        (Variables|Default|SetlastSeenPlayer (.location (Transformation|GetActorTransform _returnvalue))))
      (:OnSuccess
        (Development|PrintString "TODO: Goblin Caught Player in BP_EnemyGoblin.FollowPlayer()" true true "(R=1.000000,G=0.000000,B=0.000000,A=1.000000)")))))

(event Custom|FindRandomTarget
  (bind _outactors (Actor|GetAllActorsOfClass "/Game/AI/BP_EnemyInterestPoint.BP_EnemyInterestPoint_C"))
  (AI|AIMoveTo self (.location (Transformation|GetActorTransform (.OutItem (Utilities|Array|Random _outactors)))) 0 5.0 false
    (:OnSuccess
      (Utilities|Time|SetTimerbyEvent (delegate Custom|FindRandomTarget) 5.0 false true) ; Let the goblin sit in suffering for a minute
    )))

(event Collision|EventActorBeginOverlap
  (params (OtherActor :type Actor%20Object%20Reference)))

(event EventTick
  (params (DeltaSeconds :type Float%20%28single-precision%29))
  (if (and (not (Variables|Default|GetisSeeingPlayer)) (Utilities|Operators|NotEqual(!=) (Variables|Default|GetlastSeenPlayer) (Variables|Default|GetresetVector) 0.1)) ; If the goblin lost sight of the player,\nit will attempt to move to the last known position
    (AI|AIMoveTo self (Variables|Default|GetlastSeenPlayer) 0 5.0 false
      (:OnSuccess
        (Variables|Default|SetlastSeenPlayer (Variables|Default|GetresetVector))
        ;[1 1 1] Lost track of player, find a random spot to move to
        (Development|PrintString "Gave up on finding player!")
        (Utilities|Time|SetTimerbyEvent (delegate Custom|FindRandomTarget) 5.0 false true) ; Let the goblin sit in suffering for a minute
      ))))

(event EventBeginPlay
  (CallFunction|FindRandomTarget))

(fn ConstructionScript)